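; Sliding double door that streams World Partition Data Layers as the custom third-person character passes between two areas.
; Entry begin-overlap and exit end-overlap events use a GoingToNewArea flag to pick travel direction.
; One side loads the destination layer and plays the door timeline; the other reverses it, then unloads the layer left behind after a delay and flips the flag.
; BeginPlay also sets an initial layer to Loaded.
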(event `self.ReceiveBeginPlay`
  (`DataLayerSubsystem.SetDataLayerRuntimeState` (subsystem `DataLayerSubsystem`) (`self.In Data Layer`) "Loaded" true))

(event `self.EntryTrigger.OnComponentBeginOverlap`
  (params (OverlappedComponent :type "PrimitiveComponent Object Reference") (OtherActor :type "Actor Object Reference") (OtherComp :type "PrimitiveComponent Object Reference") (OtherBodyIndex :type Integer) (bFromSweep :type Boolean) (SweepResult :type "HitResult Structure (by ref)"))
  (cast `/Game/Blueprints/BP_ThirdPersonCharacterCustom` OtherActor)
  (if (`self.Going To New Area`)
    ;[1 1 1] Loading and Unloading Data Layers
    (`DataLayerSubsystem.SetDataLayerRuntimeStateByLabel` (subsystem `DataLayerSubsystem`) (`self.NewDataLayer`) "Loaded" true)
    (bind (_direction _newtrack_0) (`Timeline|Open Doors` :!via `PlayFromStart` :!label _label)
      (:`Update`
        (`SceneComponent.K2_SetRelativeLocation` (`self.LeftDoor`) (`KismetMathLibrary.VLerp` (0.0 -100.0 100.0) (0.0 -200.0 100.0) _newtrack_0) false false)
        (`SceneComponent.K2_SetRelativeLocation` (`self.RightDoor`) (`KismetMathLibrary.VLerp` (0.0 100.0 100.0) (0.0 200.0 100.0) _newtrack_0) false false)))
    (else
      (`|ExecutionSequence`
        (:`then_0`
          (goto _label :!via `ReverseFromEnd`))
        (:`then_1`
          (`KismetSystemLibrary.Delay` 2.0)
          (`DataLayerSubsystem.SetDataLayerRuntimeStateByLabel` (subsystem `DataLayerSubsystem`) (`self.NewDataLayer`) "Unloaded" true)
          (set `self.Going To New Area` true))))))

(event `self.ExitTrigger.OnComponentEndOverlap`
  (params (OverlappedComponent :type "PrimitiveComponent Object Reference") (OtherActor :type "Actor Object Reference") (OtherComp :type "PrimitiveComponent Object Reference") (OtherBodyIndex :type Integer))
  (cast `/Game/Blueprints/BP_ThirdPersonCharacterCustom` OtherActor)
  (if (`self.Going To New Area`)
    (`|ExecutionSequence`
      (:`then_0`
        (goto _label :!via `ReverseFromEnd`))
      (:`then_1`
        (`KismetSystemLibrary.Delay` 2.0)
        ;[1 1 1] Loading and Unloading Data Layers
        (`DataLayerSubsystem.SetDataLayerRuntimeStateByLabel` (subsystem `DataLayerSubsystem`) (`self.OldDataLayer`) "Unloaded" true)
        (set `self.Going To New Area` false)))
    (else
      (`DataLayerSubsystem.SetDataLayerRuntimeStateByLabel` (subsystem `DataLayerSubsystem`) (`self.OldDataLayer`) "Loaded" true)
      (goto _label :!via `PlayFromStart`))))

(fn `UserConstructionScript`)