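; Experimental actor that polls its Sphere component for overlapping BP_CanOfBeans actors and destroys them.
; BeginPlay starts a delayed loop that prints the overlap count, then calls DestroyActor on each can found.
; The loop repeats only after finding cans, so the first empty check ends polling for good.
; A cast to BP_CanOfBeans calling DestroyMyself is left unconnected.
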(event `self.ReceiveBeginPlay`
  (bind _overlappingactors (`PrimitiveComponent.GetOverlappingActors` (`self.Sphere`) "/Game/Blueprints/BP_CanOfBeans.BP_CanOfBeans_C"))
  (bind _returnvalue (`KismetArrayLibrary.Array_Length` _overlappingactors))
  (`KismetSystemLibrary.PrintString` "starting overlap experiment")
  (`KismetSystemLibrary.Delay` 2.0 :!label _label)
  (if (> _returnvalue 0)
    (`KismetSystemLibrary.PrintString` (`KismetStringLibrary.Concat_StrStr` "there are " (`KismetStringLibrary.Conv_IntToString` _returnvalue) "actors we are overlapping"))
    (for _array_element _overlappingactors
      (`self.K2_DestroyActor` _array_element))
    (goto _label)))

(fn `UserConstructionScript`)