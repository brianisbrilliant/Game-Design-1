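; BP_PatrolAI is a patrolling character that walks endlessly between actors tagged as town patrol points.
; On BeginPlay it gathers and shuffles those points, starts moving after a short delay, and picks a random walk speed.
; MoveToNextPoint uses AIMoveTo, then on success or failure advances a wrapping index and calls itself again after a brief delay.
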(event `self.ReceiveBeginPlay`
  (bind _outactors (`GameplayStatics.GetAllActorsOfClassWithTag` "/Script/Engine.Actor" "PatrolPoint-Town"))
  (`KismetArrayLibrary.Array_Shuffle` _outactors)
  (`KismetSystemLibrary.PrintString` (`KismetStringLibrary.Concat_StrStr` "There are " (`KismetStringLibrary.Conv_IntToString` (`KismetArrayLibrary.Array_Length` _outactors)) " patrol points"))
  (`KismetSystemLibrary.Delay` 0.2)
  (`self.MoveToNextPoint`)
  (set `CharacterMovementComponent.MaxWalkSpeed` (* (`KismetMathLibrary.RandomFloatInRange` 8.0 12.0) 25.0) (`self.CharacterMovement`)))

(event `MoveToNextPoint`
  (`|AIMoveTo` self (`self.K2_GetActorLocation` (`|GetArrayItem` (stale `self.ReceiveBeginPlay` _outactors) (`self.Index`))) null 50.0
    (:`OnSuccess`
      _)
    (:`OnFail`
      _))
  (set `self.Index` (mod (+ (`self.Index`) 1) (`KismetArrayLibrary.Array_Length` (stale `self.ReceiveBeginPlay` _outactors))))
  (`KismetSystemLibrary.Delay` 0.2)
  (`self.MoveToNextPoint`)
  (`KismetSystemLibrary.PrintString` "End of Move To Next Point"))

(fn `UserConstructionScript`)