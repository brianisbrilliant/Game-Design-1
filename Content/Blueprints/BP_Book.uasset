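; BP_Book is a readable book pickup that shows its description when the player presses E nearby.
; On BeginPlay it creates the description and "Press E" widgets, filling the former from BookDescription.
; Sphere overlap with the custom third-person character shows the prompt and enables input; leaving removes both widgets, disables input and resets the state.
; E toggles between prompt and description via the ShowPressE boolean; an unused FlipFlop remains.
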(event `self.ReceiveBeginPlay`
  (bind _returnvalue (`|CreateWidget` "/Game/Widgets/W_BookDetails.W_BookDetails_C"))
  (set `TextBlock.Text` (`self.BookDescription`) (`/Game/Widgets/W_BookDetails.Text_BookDescription` _returnvalue))
  (bind _returnvalue_2 (`|CreateWidget` "/Game/Widgets/W_PressE.W_PressE_C"))
  (`Widget.RemoveFromParent` _returnvalue_2 :!label _label)
  (`Widget.RemoveFromParent` _returnvalue)
  (`self.DisableInput` (`GameplayStatics.GetPlayerController` 0))
  (set `self.ShowPressE` true))

(event `self.Sphere.OnComponentBeginOverlap`
  (params (OverlappedComponent :type "PrimitiveComponent Object Reference") (OtherActor :type "Actor Object Reference") (OtherComp :type "PrimitiveComponent Object Reference") (OtherBodyIndex :type Integer) (bFromSweep :type Boolean) (SweepResult :type "HitResult Structure (by ref)"))
  (cast `/Game/Blueprints/BP_ThirdPersonCharacterCustom` OtherActor)
  (`UserWidget.AddToViewport` (stale `self.ReceiveBeginPlay` _returnvalue_2) 0)
  (`self.EnableInput` (`GameplayStatics.GetPlayerController` 0)))

(event `self.Sphere.OnComponentEndOverlap`
  (params (OverlappedComponent :type "PrimitiveComponent Object Reference") (OtherActor :type "Actor Object Reference") (OtherComp :type "PrimitiveComponent Object Reference") (OtherBodyIndex :type Integer))
  (cast `/Game/Blueprints/BP_ThirdPersonCharacterCustom` OtherActor)
  (goto _label))

(event `Key|E`
  (params (Key :type "Key Structure"))
  (:`Pressed`
    (if (`self.ShowPressE`)
      (`UserWidget.AddToViewport` (stale `self.ReceiveBeginPlay` _returnvalue) 0) ; book details
      (`Widget.RemoveFromParent` (stale `self.ReceiveBeginPlay` _returnvalue_2)) ; press e
      (set `self.ShowPressE` false)
      (else
        (`Widget.RemoveFromParent` (stale `self.ReceiveBeginPlay` _returnvalue))
        (`UserWidget.AddToViewport` (stale `self.ReceiveBeginPlay` _returnvalue_2) 0)
        (set `self.ShowPressE` true)))))

(fn `UserConstructionScript`)