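; A trigger volume actor that moves the game to the next streamed level when the custom third-person character enters its box.
; On overlap it records the current level name, asynchronously loads the Destination level as visible, then unloads the level by that recorded name.
; Print strings report each step or a missing destination.
; Camera repositioning logic is present but never runs, and fade-related nodes are unused.
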(event `self.Box Trigger.OnComponentBeginOverlap`
  (params (OverlappedComponent :type "PrimitiveComponent Object Reference") (OtherActor :type "Actor Object Reference") (OtherComp :type "PrimitiveComponent Object Reference") (OtherBodyIndex :type Integer) (bFromSweep :type Boolean) (SweepResult :type "HitResult Structure (by ref)"))
  (bind _returnvalue (`GameplayStatics.GetCurrentLevelName` true))
  (bind _asbp_third_person_character_custom (cast `/Game/Blueprints/BP_ThirdPersonCharacterCustom` OtherActor))
  (bind _destination (`self.Destination`) ; do we have a level to go to?
    (:`then`
      (`GameplayStatics.LoadStreamLevelBySoftObjectPtr` _destination true)
      (`KismetSystemLibrary.PrintString` "New Level is Loaded.")
      (`GameplayStatics.UnloadStreamLevel` (`KismetStringLibrary.Conv_StringToName` _returnvalue))
      (`KismetSystemLibrary.PrintString` "old level is unloaded"))
    (:`else`
      (`KismetSystemLibrary.PrintString` "No Valid Destination"))))

(fn `UserConstructionScript`)