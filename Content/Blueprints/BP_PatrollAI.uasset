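; BP_PatrollAI is an AI character that patrols between tagged actors in shuffled order.
; On BeginPlay it gathers and shuffles the points and picks a random, stepped walk speed.
; GoToPatrolPoint loops AIMoveTo with a short delay, advancing on success or failure and reshuffling after each full pass.
; A similar GoToDestination loop chases the player character, but nothing in this Blueprint starts it.
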(event `self.ReceiveBeginPlay`
  ;[1 1 1] Begin Play
  (bind _outactors (`GameplayStatics.GetAllActorsOfClassWithTag` "/Script/Engine.Actor" (`self.PatrolPointTag`)))
  (`KismetSystemLibrary.PrintString` (`KismetStringLibrary.Concat_StrStr` "There are " (`KismetStringLibrary.Conv_IntToString` (`KismetArrayLibrary.Array_Length` _outactors)) " patrol points."))
  (`KismetArrayLibrary.Array_Shuffle` _outactors)
  (set `CharacterMovementComponent.MaxWalkSpeed` (`KismetMathLibrary.Conv_IntToDouble` (* (`KismetMathLibrary.RandomIntegerInRange` 12 16) 25)) (`self.CharacterMovement`))
  (`self.GoToPatrolPoint`))

(event `GoToPatrolPoint`
  ;[1 1 1] Patrol
  (`|AIMoveTo` self (`self.K2_GetActorLocation` (`|GetArrayItem` (stale `self.ReceiveBeginPlay` _outactors) (`self.CurrentPatrolPoint`))) null 110.0 ; Move ourselves to the player's location,\nconstantly updating, and stopping 2 meters away.
    (:`OnSuccess`
      (`KismetSystemLibrary.PrintString` "Arrived at Desitination"))
    (:`OnFail`
      (`KismetSystemLibrary.PrintString` "Failed to get to Destination." true true (struct :`R` 1.0 :`G` 0.044287 :`B` 0.060866 :`A` 1.0))))
  (bind _result (`/Engine/EditorBlueprintResources/StandardMacros.IncrementInt` (`self.CurrentPatrolPoint`)) ; Increment Int
    (:`  `
      (if (>= _result (`KismetArrayLibrary.Array_Length` (stale `self.ReceiveBeginPlay` _outactors)))
        (set `self.CurrentPatrolPoint` 0)
        (`KismetArrayLibrary.Array_Shuffle` (stale `self.ReceiveBeginPlay` _outactors)))
      (`KismetSystemLibrary.Delay` 1.0)
      (`self.GoToPatrolPoint`))))

(event `GoToDestination`
  ;[1 1 1] Go To Player
  (`|AIMoveTo` self (0.0 0.0 0.0) (`GameplayStatics.GetPlayerCharacter` 0) 50.0 ; Move ourselves to the player's location,\nconstantly updating, and stopping 2 meters away.
    (:`OnSuccess`
      (`KismetSystemLibrary.PrintString` "Arrived at Desitination"))
    (:`OnFail`
      (`KismetSystemLibrary.PrintString` "Failed to get to Destination." true true (struct :`R` 1.0 :`G` 0.044287 :`B` 0.060866 :`A` 1.0))))
  (`KismetSystemLibrary.Delay` 1.0)
  (`self.GoToDestination`))

(fn `UserConstructionScript`)